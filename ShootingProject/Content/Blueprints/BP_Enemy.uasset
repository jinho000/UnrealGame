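; BP_Enemy is an enemy that flies in a straight line and ends the game on touching BP_Player.
; BeginPlay aims it once at the player when a random roll is at least TraceRate; otherwise it keeps its forward direction.
; Tick moves it along that fixed direction by MoveSpeed, without sweep.
; Player overlap spawns an explosion, shows the game-over widget and cursor, pauses the game and destroys the enemy.
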(event `self.ReceiveBeginPlay`
  ;[1 1 1] 35%확률로 플레이어 위치로 갈지 설정
  (if (<= (`self.TraceRate`) (`KismetMathLibrary.RandomFloatInRange` 0.0 1.0))
    (bind _returnvalue (`GameplayStatics.GetActorOfClass` "/Game/Blueprints/BP_Player.BP_Player_C"))
    (`/Engine/EditorBlueprintResources/StandardMacros.IsValid` _returnvalue
      (:`Is Valid`
        (bind _output_get (set `self.Direction` (`KismetMathLibrary.Normal` (- (`self.K2_GetActorLocation` _returnvalue) (`self.K2_GetActorLocation`)))))
        ;[1 1 1] 처음에 한번 플레이어 방향으로 회전
        (`self.K2_SetActorRotation` (`KismetMathLibrary.MakeRotFromXZ` _output_get (`self.GetActorUpVector`)))))
    (else
      (set `self.Direction` (`self.GetActorForwardVector`)))))

(event `self.ReceiveActorBeginOverlap`
  (params (OtherActor :type "Actor Object Reference"))
  (cast `/Game/Blueprints/BP_Player` OtherActor)
  (`GameplayStatics.SpawnEmitterAtLocation` "/Game/StarterContent/Particles/P_Explosion.P_Explosion" (`self.K2_GetActorLocation`))
  (bind _returnvalue (`|CreateWidget` "/Game/UI/BP_GameOverWidget.BP_GameOverWidget_C"))
  (`UserWidget.AddToViewport` _returnvalue 0)
  (set `PlayerController.bShowMouseCursor` true (`GameplayStatics.GetPlayerController` 0))
  (`GameplayStatics.SetGamePaused` true)
  (`self.K2_DestroyActor`))

(event `self.ReceiveTick`
  (params (DeltaSeconds :type "Float (single-precision)"))
  (`self.K2_SetActorLocation` (+ (`self.K2_GetActorLocation`) (* DeltaSeconds (* (`self.MoveSpeed`) (`self.Direction`))))))

(fn `UserConstructionScript`)