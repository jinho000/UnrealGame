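; BP_Player is the player actor that moves in a plane and fires bullets.
; Each tick it builds a direction from horizontal and vertical axis inputs on Y and Z, normalizes it, and moves by MoveSpeed times delta seconds without sweeping.
; The Fire action spawns a BP_Bullet at the FirePosition component's transform and plays a blaster sound.
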(event `InputAction|Fire`
  (params (Key :type "Key Structure"))
  ;[1 1 1] 입력감지시 이벤트 실행
  (:`Pressed`
    (`|SpawnActorFromClass` "/Game/Blueprints/BP_Bullet.BP_Bullet_C" (`SceneComponent.K2_GetComponentToWorld` (`self.FirePosition`)) "AlwaysSpawn" "OverrideRootScale" null null)
    (`GameplayStatics.PlaySound2D` "/Game/Audio/star-wars-blaster.star-wars-blaster" 1.0 1.0 0.0 null null)))

(event `self.ReceiveTick`
  (params (DeltaSeconds :type "Float (single-precision)"))
  (`self.K2_SetActorLocation` (+ (* DeltaSeconds (* (`KismetMathLibrary.Normal` (`KismetMathLibrary.MakeVector` 0.0 (`self.GetInputAxisValue`) (`self.GetInputAxisValue`))) (`self.moveSpeed`))) (`self.K2_GetActorLocation`))))

(fn `UserConstructionScript`)